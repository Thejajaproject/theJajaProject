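; Shared two-player camera actor that becomes the first player controller's view target and keeps both players framed.
; Each tick it centers above the players' midpoint, scaling spring arm length and pitch with their separation.
; A reference point offset toward the player nearer the camera drives yaw, turning when Player1 strays past a minimum distance.
; The look-at and alternate rotation functions are abandoned and never run.
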(event `self.ReceiveBeginPlay`
  (`PlayerController.SetViewTargetWithBlend` (`GameplayStatics.GetPlayerController` 0) self 0.0 "VTBlend_Linear" 0.0 false))

(event `self.ReceiveTick`
  (params (DeltaSeconds :type "Float (single-precision)"))
  ;[1 1 1] If both players are already defined
  (if (and (!= (`self.Player1`) null) (!= (`self.Player2`) null))
    ;[1 1 1] Set players references
    (`self.SetPlayerReference`)
    ;[1 1 1] Move camera between players
    (`self.SetCameraPosition`)
    ;[1 1 1] Rotate camera between players
    (`self.RotateBetweenPlayers`)
    (else
      (`/Engine/EditorBlueprintResources/StandardMacros.DoOnce` false
        (:`Completed`
          (`KismetSystemLibrary.PrintText` "There is a player lacking! Please set all the players!" true true (struct :`R` 0.21875 :`G` 0.057111 :`B` 0.115035 :`A` 1.0)))))))

(fn `CalculateLookAtFuction`
  (params (Player1 :type "Actor Object Reference") (Player2 :type "Actor Object Reference"))
  (bind _returnvalue (`self.K2_GetActorLocation` Player1))
  (bind _returnvalue_2 (`self.K2_GetActorLocation` Player2))
  (bind _returnvalue_3 (`KismetMathLibrary.FClamp` (`self.GlobalDistanceFactor`)))
  (`SceneComponent.K2_SetRelativeRotation` (`self.SpringArm`) (`KismetMathLibrary.MakeRotator` (* (.roll (`KismetMathLibrary.RInterpTo` (`SceneComponent.RelativeRotation` (`self.SpringArm`)) (select `bool` (> (`self.CameraMovementMultiplier`) 0.0) :`false` (`KismetMathLibrary.FindLookAtRotation` _returnvalue_2 _returnvalue) :`true` (`KismetMathLibrary.FindLookAtRotation` _returnvalue _returnvalue_2)) (`GameplayStatics.GetWorldDeltaSeconds`) (`self.LookAtSpeed`))) _returnvalue_3) (* (.pitch (`KismetMathLibrary.RInterpTo` (`SceneComponent.RelativeRotation` (`self.SpringArm`)) (select `bool` (> (`self.CameraMovementMultiplier`) 0.0) :`false` (`KismetMathLibrary.FindLookAtRotation` _returnvalue_2 _returnvalue) :`true` (`KismetMathLibrary.FindLookAtRotation` _returnvalue _returnvalue_2)) (`GameplayStatics.GetWorldDeltaSeconds`) (`self.LookAtSpeed`))) _returnvalue_3)) false false))

(fn `CalculateRotationFunction`
  (params (`Player Actor` :type "Actor Object Reference") (`Player Reference` :type "SceneComponent Object Reference"))
  (bind _returnvalue (`self.K2_GetActorLocation` `Player Actor`))
  (bind _returnvalue_2 (`SceneComponent.K2_GetComponentLocation` `Player Reference`))
  (bind _returnvalue_3 (`KismetMathLibrary.GetRightVector` (`SceneComponent.K2_GetComponentRotation` `Player Reference`)))
  (bind _returnvalue_4 (`KismetMathLibrary.GetDirectionUnitVector` _returnvalue _returnvalue_2))
  (bind _returnvalue_5 (`KismetMathLibrary.VSize` (- _returnvalue _returnvalue_2)))
  (if (>= _returnvalue_5 (`self.MinimumRightDistance`))
    (`SceneComponent.K2_AddWorldRotation` (`self.DefaultSceneRoot`) (`KismetMathLibrary.MakeRotator` 0.0 0.0 (* (`GameplayStatics.GetWorldDeltaSeconds`) (* (* (`self.CameraMovementMultiplier`) (`KismetMathLibrary.SelectFloat` -1.0 1.0 (> (`KismetMathLibrary.DegAcos` (/ (`KismetMathLibrary.Dot_VectorVector` _returnvalue_3 _returnvalue_4) (* (`KismetMathLibrary.VSize` _returnvalue_4) (`KismetMathLibrary.VSize` _returnvalue_3)))) 90.0))) (/ (- _returnvalue_5 (`self.MinimumRightDistance`)) (`self.RotationDelay`))))) false false))
  (`SceneComponent.K2_SetRelativeRotation` (`self.SpringArm`) (`KismetMathLibrary.MakeRotator` 0.0 (* -5.0 (`self.GlobalDistanceFactor`))) false false))

(fn `RotateBetweenPlayers`
  (bind _playersreference (`self.PlayersReference`))
  (bind _returnvalue (`self.K2_GetActorLocation` (`self.Player1`)))
  (bind _returnvalue_2 (`SceneComponent.K2_GetComponentLocation` _playersreference))
  (bind _returnvalue_3 (`KismetMathLibrary.GetRightVector` (`SceneComponent.K2_GetComponentRotation` _playersreference)))
  (bind _returnvalue_4 (`KismetMathLibrary.GetDirectionUnitVector` _returnvalue _returnvalue_2))
  (bind _returnvalue_5 (`KismetMathLibrary.VSize` (- _returnvalue _returnvalue_2)))
  (if (>= _returnvalue_5 (`self.MinimumRightDistance`))
    (`SceneComponent.K2_AddWorldRotation` (`self.DefaultSceneRoot`) (`KismetMathLibrary.MakeRotator` 0.0 0.0 (* (`GameplayStatics.GetWorldDeltaSeconds`) (* (* (`self.CameraMovementMultiplier`) (`KismetMathLibrary.SelectFloat` -1.0 1.0 (> (`KismetMathLibrary.DegAcos` (/ (`KismetMathLibrary.Dot_VectorVector` _returnvalue_3 _returnvalue_4) (* (`KismetMathLibrary.VSize` _returnvalue_4) (`KismetMathLibrary.VSize` _returnvalue_3)))) 90.0))) (/ (- _returnvalue_5 (`self.MinimumRightDistance`)) (`self.RotationDelay`))))) false false))
  (`SceneComponent.K2_SetRelativeRotation` (`self.SpringArm`) (`KismetMathLibrary.MakeRotator` 0.0 (* (`KismetMathLibrary.Lerp` (`self.MaximunCameraRotation`) (`self.MinimumCameraRotation`) (`self.GlobalDistanceFactor`)) -1.0)) false false))

(fn `SetCameraPosition`
  (bind _springarmbasedistance (`self.SpringArmBaseDistance`))
  (bind _springarm (`self.SpringArm`))
  (bind _returnvalue (`self.K2_GetActorLocation` (`self.Player2`)))
  (bind _returnvalue_2 (`self.K2_GetActorLocation` (`self.Player1`)))
  (bind _returnvalue_location (`KismetMathLibrary.BreakTransform` (`SceneComponent.GetSocketTransform` _springarm "None" "RTS_Component")))
  (bind (_returnvalue_x _returnvalue_y) (`KismetMathLibrary.BreakVector` (- _returnvalue _returnvalue_2)))
  (set `self.GlobalDistanceFactor` (`KismetMathLibrary.FClamp` (/ (`KismetMathLibrary.VSize` (- _returnvalue _returnvalue_2)) 1200.0)))
  (`SceneComponent.K2_SetWorldLocation` (`self.DefaultSceneRoot`) (+ (/ (+ _returnvalue_2 _returnvalue) 2.0) (`KismetMathLibrary.MakeVector` 0.0 0.0 (`self.Height`))) false false)
  (set `SpringArmComponent.TargetArmLength` (+ (`KismetMathLibrary.VSize` (/ (`KismetMathLibrary.MakeVector` _returnvalue_x _returnvalue_y) 2.0)) (`KismetMathLibrary.Lerp` _springarmbasedistance (+ _springarmbasedistance (`self.SpringArmExtraDistance`)) (`self.GlobalDistanceFactor`))) (`self.SpringArm`))
  (set `self.SpringDifference` (/ (`KismetMathLibrary.FClamp` (/ (+ (`SpringArmComponent.TargetArmLength` _springarm) (.x _returnvalue_location)) (`self.WallAdjustment`)) 0.0 10.0) 10.0)))

(fn `SetPlayerReference`
  (bind _returnvalue (`self.K2_GetActorLocation` (`self.Player2`)))
  (bind _returnvalue_2 (`self.K2_GetActorLocation` (`self.Player1`)))
  (bind _returnvalue_3 (`SceneComponent.K2_GetComponentLocation` (`self.Camera`)))
  (bind _returnvalue_4 (/ (`KismetMathLibrary.VSize` (- _returnvalue_2 _returnvalue)) 2.0))
  (if (> (`KismetMathLibrary.VSize` (- _returnvalue _returnvalue_3)) (`KismetMathLibrary.VSize` (- _returnvalue_2 _returnvalue_3)))
    (`SceneComponent.K2_SetRelativeLocation` (`self.PlayersReference`) (`KismetMathLibrary.MakeVector` (* _returnvalue_4 -1.0)) false false)
    (set `self.CameraMovementMultiplier` 1.0)
    (else
      (`SceneComponent.K2_SetRelativeLocation` (`self.PlayersReference`) (`KismetMathLibrary.MakeVector` _returnvalue_4) false false)
      (set `self.CameraMovementMultiplier` -1.0))))

(fn `UserConstructionScript`)